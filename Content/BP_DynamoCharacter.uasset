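; BP_DynamoCharacter is a character Blueprint that tints human players with their configured color.
; On BeginPlay it waits briefly for the pawn to initialize, then checks whether its controller belongs to a human player.
; If so, it looks up that player's color in the DynamoGameInstance PlayerConfigs by controller ID and applies it through a dynamic material on the Sphere component.
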(event `self.ReceiveBeginPlay`
  (bind (_outisplayerhuman _outplayercontrollerid) (`self.K2_GetPlayerControllerId`))
  (`KismetSystemLibrary.Delay` 0.1) ; Make sure the pawn has initialized
  (if _outisplayerhuman
    (bind _asdynamo_game_instance (cast `DynamoGameInstance` (`GameplayStatics.GetGameInstance`)))
    (bind _returnvalue (`PrimitiveComponent.CreateDynamicMaterialInstance` (`self.Sphere`) 0 null "None"))
    (bind (_output_name _output_color) (break `PlayerConfiguration` (`|GetArrayItem` (`DynamoGameInstance.PlayerConfigs` _asdynamo_game_instance) _outplayercontrollerid)))
    (`MaterialInstanceDynamic.SetVectorParameterValue` _returnvalue "Color" (`KismetMathLibrary.Conv_ColorToLinearColor` _output_color))))

(fn `UserConstructionScript`)